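; BP_SteamSeshComp is a Steam lobby component that manages a player controller's pause menu and input focus.
; FocusGameOnly sets game-only input, hides the cursor and, for local controllers, creates and caches WBP_PauseMenu if none is valid.
; The IA_OpenPauseMenu input toggles that cached widget on Completed, switching cursor visibility and game-only or game-and-UI input, and relies on FocusGameOnly having created it.
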(event Input|EnhancedActionEvents|EnhancedInputActionIA_OpenPauseMenu
  (params (ActionValue :type Boolean) (ElapsedSeconds :type Float%20%28double-precision%29) (TriggeredSeconds :type Float%20%28double-precision%29) (InputAction :type Input%20Action%20Object%20Reference :default "/Game/Lobby/Steam/Input/IA_OpenPauseMenu.IA_OpenPauseMenu"))
  (:Completed
    (if (Widget|IsVisible (Variables|Default|GetUI_PauseMenu))
      (Widget|RemovefromParent (Variables|Default|GetUI_PauseMenu))
      (Variables|/Script/Engine.PlayerController|SetbShowMouseCursor (Variables|Default|GetPlayer%20Controller) false)
      (Input|SetInputModeGameOnly (Variables|Default|GetPlayer%20Controller) false)
      (else
        (UserInterface|Viewport|AddtoViewport (Variables|Default|GetUI_PauseMenu) 0)
        (Variables|/Script/Engine.PlayerController|SetbShowMouseCursor (Variables|Default|GetPlayer%20Controller) true)
        (Input|SetInputModeGameandUI (Variables|Default|GetPlayer%20Controller) (Variables|Default|GetUI_PauseMenu) "DoNotLock" true false)))))

(event EventBeginPlay)

(event EventTick
  (params (DeltaSeconds :type Float%20%28single-precision%29)))

(fn FocusGameOnly
  (Input|SetInputModeGameOnly (Variables|Default|GetPlayer%20Controller) false)
  (Variables|/Script/Engine.PlayerController|SetbShowMouseCursor (Variables|Default|GetPlayer%20Controller) false)
  (if (Pawn|IsLocalController (Variables|Default|GetPlayer%20Controller))
    (Utilities|IsValid (Variables|Default|GetUI_PauseMenu)
      (:Is%20Not%20Valid
        (bind _returnvalue (UserInterface|CreateWidget "/Game/Lobby/Steam/UI/WBP_PauseMenu.WBP_PauseMenu_C"))
        (Variables|Default|SetUI_PauseMenu _returnvalue)))))