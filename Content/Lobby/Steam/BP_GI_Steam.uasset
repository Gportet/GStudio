(event Custom|CreateNewSession
  (params (PlayerController :type Player%20Controller%20Object%20Reference) (Nb_Connections :type Integer))
  (|AdvancedSession 0 PlayerController Nb_Connections 0 false true false true true false false false true false true
    (:OnSuccess
      (Utilities|FlowControl|Delay 0.2)
      ;[0.15 0.15 0.15 0.5] A changer !
      (Game|OpenLevel(byObjectReference) "/Game/Variant_Combat/Lvl_Combat.Lvl_Combat" true "?listen"))
    (:OnFailure
      (Development|PrintString "Session Creation failed " true true "(R=1.000000,G=0.000000,B=0.000000,A=1.000000)"))))

(event EventOnSessionInviteAccepted
  (params (LocalPlayerNum :type Integer) (PersonInvited :type BP%20Unique%20Net%20Id%20Structure) (SessionToJoin :type Blueprint%20Session%20Result%20Structure%20%28by%20ref%29))
  (|JoinSession (Game|GetPlayerController 0) SessionToJoin
    (:OnFailure
      (Development|PrintString "Failed Join Session" true true "(R=1.000000,G=0.000000,B=0.000000,A=1.000000)"))))

(event EventHandleNetworkError
  (params (FailureType :type ENetworkFailure%20Enum :default "NetDriverAlreadyExists") (bIsServer :type Boolean))
  (|DestroySession (Game|GetPlayerController 0)))